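; BP_Star is a collectible star that hovers via a timeline lerping its Z position by Height.
; Sphere overlap starts the TL_GetStar timeline, and ending overlap stops it, so pickup waits for the timeline's Get Star event.
; That event loops over top-level BI_Star widgets, incrementing BP_Player's StarNum inside the loop, passing the count, playing a sound and destroying the star.
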(event `self.ReceiveBeginPlay`
  (`self.Float`))

(event `Float`
  (bind (_returnvalue_x _returnvalue_y _returnvalue_z) (`KismetMathLibrary.BreakVector` (`SceneComponent.K2_GetComponentLocation` (`self.Star`))))
  (set `self.PositionZ` _returnvalue_z)
  (bind (_direction _track_positionz) (`Timeline|时间轴`)
    (:`Update`
      (`SceneComponent.K2_SetWorldLocation` (`self.Star`) (`KismetMathLibrary.MakeVector` _returnvalue_x _returnvalue_y (`KismetMathLibrary.Lerp` (`self.PositionZ`) (+ (`self.PositionZ`) (`self.Height`)) _track_positionz)) false false))))

(event `self.Sphere.OnComponentBeginOverlap`
  (params (OverlappedComponent :type "PrimitiveComponent Object Reference") (OtherActor :type "Actor Object Reference") (OtherComp :type "PrimitiveComponent Object Reference") (OtherBodyIndex :type Integer) (bFromSweep :type Boolean) (SweepResult :type "HitResult Structure (by ref)"))
  (`Timeline|TL_GetStar` :!via `PlayFromStart` :!label _label
    (:`Get Star`
      (bind _foundwidgets (`WidgetBlueprintLibrary.GetAllWidgetsWithInterface` "/Game/Widget/BI_Star.BI_Star_C" true))
      (for _array_element _foundwidgets
        (bind _asbp_player (cast `/Game/Player/BP_Player` (`GameplayStatics.GetPlayerCharacter` 0)))
        (bind _result (`/Engine/EditorBlueprintResources/StandardMacros.IncrementInt` (`/Game/Player/BP_Player.StarNum` _asbp_player))
          (:`  `
            (message `/Game/Widget/BI_Star.Pass Star Num` _array_element (`KismetTextLibrary.Conv_IntToText` _result))
            (`GameplayStatics.PlaySound2D` "/Game/SoundEffects/SFX_GetStar.SFX_GetStar" 1.0 1.0 0.0 null null)
            (`self.K2_DestroyActor`)))))))

(event `self.Sphere.OnComponentEndOverlap`
  (params (OverlappedComponent :type "PrimitiveComponent Object Reference") (OtherActor :type "Actor Object Reference") (OtherComp :type "PrimitiveComponent Object Reference") (OtherBodyIndex :type Integer))
  (goto _label :!via `Stop`))

(fn `UserConstructionScript`)