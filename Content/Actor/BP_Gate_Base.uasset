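; BP_Gate_Base is a base gate actor that can slide its platform along its local X axis.
; On BeginPlay, if Move is set, Transverse waits for DelayTime multiplied by DelayOrder, which lets gate instances start in a staggered sequence.
; A timeline then plays from the start, and its Overturn track lerps BasePlat's relative X location between A and B.
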(event `self.ReceiveBeginPlay`
  (if (`self.Move?`)
    (`self.Transverse`)))

(event `Transverse`
  (`KismetSystemLibrary.Delay` (* (`self.DelayTime`) (`self.DelayOrder`)))
  (bind (_direction _overturn) (`Timeline|时间轴` :!via `PlayFromStart`)
    (:`Update`
      (`SceneComponent.K2_SetRelativeLocation` (`self.BasePlat`) (`KismetMathLibrary.MakeVector` (`KismetMathLibrary.Lerp` (`self.A`) (`self.B`) _overturn)) false false))))

(fn `UserConstructionScript`)