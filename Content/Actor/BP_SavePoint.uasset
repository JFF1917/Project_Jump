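; BP_SavePoint is a checkpoint that also serves as a one-shot moving platform between levels.
; Entering Box stores BasePlat's position and rotation as the player's respawn point, sets a BGM state and plays a save sound.
; Entering MoveBox enables four walls' collision, then a Timeline slides and yaws BasePlat by offsets chosen from Type.
; On arrival, it updates the respawn point and disables the walls' collision.
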(event `self.ReceiveBeginPlay`)

(event `self.Box.OnComponentBeginOverlap`
  (params (OverlappedComponent :type "PrimitiveComponent Object Reference") (OtherActor :type "Actor Object Reference") (OtherComp :type "PrimitiveComponent Object Reference") (OtherBodyIndex :type Integer) (bFromSweep :type Boolean) (SweepResult :type "HitResult Structure (by ref)"))
  (`/Engine/EditorBlueprintResources/StandardMacros.DoOnce` false
    (:`Completed`
      (bind _outputpin (`self.SetRebornPlayer`))
      (set `/Game/Player/BP_Player.BGMState` "NewEnumerator2" _outputpin)
      (`GameplayStatics.PlaySound2D` "/Game/SoundEffects/SFX_Save.SFX_Save" 1.0 1.0 0.0 null null))))

(event `self.MoveBox.OnComponentBeginOverlap`
  (params (OverlappedComponent :type "PrimitiveComponent Object Reference") (OtherActor :type "Actor Object Reference") (OtherComp :type "PrimitiveComponent Object Reference") (OtherBodyIndex :type Integer) (bFromSweep :type Boolean) (SweepResult :type "HitResult Structure (by ref)"))
  (`/Engine/EditorBlueprintResources/StandardMacros.DoOnce` false
    (:`Completed`
      (if (`KismetStringLibrary.EqualEqual_StrStr` (`self.Type`) "ToNext")
        (set `self.X` 28285.0)
        (set `self.Y` 0.0)
        (set `self.Rotation Z` 0.0)
        (`PrimitiveComponent.SetCollisionEnabled` (`self.Wall2`) "QueryAndPhysics" :!label _label)
        (`PrimitiveComponent.SetCollisionEnabled` (`self.Wall1`) "QueryAndPhysics")
        (`PrimitiveComponent.SetCollisionEnabled` (`self.Wall3`) "QueryAndPhysics")
        (`PrimitiveComponent.SetCollisionEnabled` (`self.Wall4`) "QueryAndPhysics")
        (`KismetSystemLibrary.Delay` 0.4)
        (bind (_direction _move _rotate) (`Timeline|时间轴` :!via `PlayFromStart`)
          (:`Update`
            (`SceneComponent.K2_SetRelativeLocation` (`self.BasePlat`) (`KismetMathLibrary.MakeVector` (`KismetMathLibrary.Lerp` 0.0 (`self.X`) _move) (`KismetMathLibrary.Lerp` 0.0 (`self.Y`) _move)) false false)
            (`SceneComponent.K2_SetRelativeRotation` (`self.BasePlat`) (`KismetMathLibrary.MakeRotator` 0.0 0.0 (`KismetMathLibrary.Lerp` 0.0 (`self.Rotation Z`) _rotate)) false false))
          (:`Finished`
            (`self.SetRebornPlayer`)
            (`PrimitiveComponent.SetCollisionEnabled` (`self.Wall2`) "NoCollision")
            (`PrimitiveComponent.SetCollisionEnabled` (`self.Wall1`) "NoCollision")
            (`PrimitiveComponent.SetCollisionEnabled` (`self.Wall3`) "NoCollision")
            (`PrimitiveComponent.SetCollisionEnabled` (`self.Wall4`) "NoCollision")))
        (elif (`KismetStringLibrary.EqualEqual_StrStr` (`self.Type`) "ToLevel01")
          (set `self.X` 20340.0)
          (set `self.Y` 0.0)
          (set `self.Rotation Z` 45.0)
          (goto _label)
          (elif (`KismetStringLibrary.EqualEqual_StrStr` (`self.Type`) "ToLevel05")
            (set `self.X` 28295.0)
            (set `self.Y` 0.0)
            (set `self.Rotation Z` -45.0)
            (goto _label)))))))

(fn `SetRebornPlayer`
  (returns (OutputPin :type "/Game/Player/BP_Player Object Reference"))
  (bind (_returnvalue_x _returnvalue_y _returnvalue_z) (`KismetMathLibrary.BreakVector` (`SceneComponent.K2_GetComponentLocation` (`self.BasePlat`))))
  (bind _asbp_player (cast `/Game/Player/BP_Player` (`GameplayStatics.GetPlayerCharacter` 0))
    (:`then`
      (set `/Game/Player/BP_Player.RebornPoint` (`KismetMathLibrary.MakeVector` _returnvalue_x _returnvalue_y (+ _returnvalue_z 155.0)) _asbp_player)
      (set `/Game/Player/BP_Player.RebornRotation` (`SceneComponent.K2_GetComponentRotation` (`self.BasePlat`)) _asbp_player))
    (:`CastFailed`
      _))
  (return _asbp_player))

(fn `UserConstructionScript`)