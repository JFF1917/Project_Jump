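; BP_Seesaw_Base is an obstacle base that slides along local X and knocks the player away on contact.
; On BeginPlay, a delay scaled by DelayOrder staggers the start of the SizeSmall timeline, which drives the obstacle's relative location.
; Capsule overlap compares player and obstacle forward vectors to choose a push direction opposing the player's approach.
; It then launches the player with a weighted horizontal push and fixed lift, and calls DeleteIMCPlayerMove.
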(event `self.ReceiveBeginPlay`
  (`self.Transverse`))

(event `Transverse`
  (bind _returnvalue (`SceneComponent.GetRelativeTransform` (`self.Obstacle`)))
  (`KismetSystemLibrary.Delay` (* (`self.DelayTime`) (`self.DelayOrder`)))
  (set `self.Location Y` (.y (.location _returnvalue)))
  (set `self.Location Z` (.z (.location _returnvalue)))
  (bind (_direction _overturn) (`Timeline|SizeSmall` :!via `PlayFromStart`)
    (:`Update`
      (`SceneComponent.K2_SetRelativeLocation` (`self.Obstacle`) (`KismetMathLibrary.MakeVector` (`KismetMathLibrary.Lerp` -600.0 600.0 _overturn) (`self.Location Y`) (`self.Location Z`)) false false))))

(event `self.Capsule.OnComponentBeginOverlap`
  (params (OverlappedComponent :type "PrimitiveComponent Object Reference") (OtherActor :type "Actor Object Reference") (OtherComp :type "PrimitiveComponent Object Reference") (OtherBodyIndex :type Integer) (bFromSweep :type Boolean) (SweepResult :type "HitResult Structure (by ref)"))
  (bind _bp_player (`self.BP_Player`))
  (bind (_returnvalue_x _returnvalue_y) (`KismetMathLibrary.BreakVector` (* (+ (* (`self.ObstacleBackward`) (`self.ObstacleWeight`)) (`self.PlayerForward`)) (`self.VelocityXYRate`))))
  (bind (_returnvalue_x_2 _returnvalue_y_2) (`KismetMathLibrary.BreakVector` (* (+ (* (`self.ObstacleForward`) (`self.ObstacleWeight`)) (`self.PlayerForward`)) (`self.VelocityXYRate`))))
  (`self.Get Obstacle Forward Backward`)
  (bind _asbp_player (cast `/Game/Player/BP_Player` OtherActor))
  (set `self.BP_Player` _asbp_player)
  (set `self.PlayerForward` (`self.GetActorForwardVector` _asbp_player))
  ;[0 0 0] 判定角色接近朝向
  (if (> (`KismetMathLibrary.VSize` (- (`self.ObstacleForward`) (`self.PlayerForward`))) 1.0)
    (`Character.LaunchCharacter` _bp_player (`KismetMathLibrary.MakeVector` _returnvalue_x_2 _returnvalue_y_2 1200.0) true true)
    (else
      (`Character.LaunchCharacter` _bp_player (`KismetMathLibrary.MakeVector` _returnvalue_x _returnvalue_y 1200.0) true true)))
  (`/Game/Player/BP_Player.Delete IMC_PlayerMove` _bp_player))

(fn `Get Obstacle Forward Backward`
  (bind _output_get (set `self.ObstacleForward` (`SceneComponent.GetForwardVector` (`self.Obstacle`))))
  (set `self.ObstacleBackward` (- (0.0 0.0 0.0) _output_get)))

(fn `UserConstructionScript`)