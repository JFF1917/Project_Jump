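; BP_Rover_Base is an actor that swings its BasePlat component through a 120-degree pitch arc while holding a fixed roll.
; On BeginPlay it waits DelayTime multiplied by DelayOrder, which allows staggered starts between instances.
; IsForward then picks one of two timelines, whose rotation track drives a Lerp between the arc's limits in opposite directions.
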(event `self.ReceiveBeginPlay`
  (`self.Rotate`))

(event `Rotate`
  (`KismetSystemLibrary.Delay` (* (`self.DelayTime`) (`self.DelayOrder`)))
  (if (`self.IsForward?`)
    (bind (_direction _track_rotation) (`Timeline|时间轴`)
      (:`Update`
        (`SceneComponent.K2_SetRelativeRotation` (`self.BasePlat`) (`KismetMathLibrary.MakeRotator` 90.0 (`KismetMathLibrary.Lerp` -60.0 60.0 _track_rotation)) false false)))
    (else
      (bind (_direction_2 _track_rotation_2) (`Timeline|时间轴_0`)
        (:`Update`
          (`SceneComponent.K2_SetRelativeRotation` (`self.BasePlat`) (`KismetMathLibrary.MakeRotator` 90.0 (`KismetMathLibrary.Lerp` 60.0 -60.0 _track_rotation_2)) false false))))))

(fn `UserConstructionScript`)