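; BP_TwoTone_Base is a base actor whose mesh changes over successive Box overlaps, counting InitialState down from 3.
; Each step rescales the mesh, decrements the state and flips the Type boolean; at 1, another overlap hides it and ending overlap disables mesh collision.
; After a flip, it adds instances with Type set to TypeValue, hiding one BP_Obstacle's mesh when that equals the loop's array index.
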(event `self.ReceiveBeginPlay`
  (bind (_returnvalue_location _returnvalue_rotation) (`KismetMathLibrary.BreakTransform` (`SceneComponent.K2_GetComponentToWorld` (`self.StaticMesh`))))
  (if (== (`self.InitialState`) 2)
    (`SceneComponent.K2_SetWorldTransform` (`self.StaticMesh`) (`KismetMathLibrary.MakeTransform` _returnvalue_location _returnvalue_rotation (`self.Scale1`)) false false)
    (elif (== (`self.InitialState`) 1)
      (`SceneComponent.K2_SetWorldTransform` (`self.StaticMesh`) (`KismetMathLibrary.MakeTransform` _returnvalue_location _returnvalue_rotation (`self.Scale2`)) false false))))

(event `self.Box.OnComponentBeginOverlap`
  (params (OverlappedComponent :type "PrimitiveComponent Object Reference") (OtherActor :type "Actor Object Reference") (OtherComp :type "PrimitiveComponent Object Reference") (OtherBodyIndex :type Integer) (bFromSweep :type Boolean) (SweepResult :type "HitResult Structure (by ref)"))
  (bind (_returnvalue_location _returnvalue_rotation) (`KismetMathLibrary.BreakTransform` (`SceneComponent.K2_GetComponentToWorld` (`self.StaticMesh`))))
  (if (== (`self.InitialState`) 3)
    (`SceneComponent.K2_SetWorldTransform` (`self.StaticMesh`) (`KismetMathLibrary.MakeTransform` _returnvalue_location _returnvalue_rotation (`self.Scale1`)) false false)
    (`/Engine/EditorBlueprintResources/StandardMacros.DecrementInt` (`self.InitialState`) :!label _label
      (:`  `
        (if (`self.Type`)
          (set `self.Type` false)
          (else
            (set `self.Type` true)))
        (bind _outactors (`GameplayStatics.GetAllActorsOfClass` "BP_TwoTone_Base_C"))
        (bind _output_get (set `self.Out Actors` _outactors))
        (for (_array_element _array_index) _output_get
          (if (`/Game/Actor/Old/BP_TwoTone_Base.Type` _array_element)
            (`/Engine/EditorBlueprintResources/StandardMacros.IncrementInt` (`self.TypeValue`))))
        (if (== _array_index (`self.TypeValue`))
          (bind _returnvalue (`GameplayStatics.GetActorOfClass` "/Game/Actor/Old/BP_Obstacle.BP_Obstacle_C"))
          (`SceneComponent.SetVisibility` (`/Game/Actor/Old/BP_Obstacle.StaticMesh` _returnvalue) false true))))
    (elif (== (`self.InitialState`) 2)
      (`SceneComponent.K2_SetWorldTransform` (`self.StaticMesh`) (`KismetMathLibrary.MakeTransform` _returnvalue_location _returnvalue_rotation (`self.Scale2`)) false false)
      (goto _label)
      (else
        (`SceneComponent.SetVisibility` (`self.StaticMesh`) false true)))))

(event `self.Box.OnComponentEndOverlap`
  (params (OverlappedComponent :type "PrimitiveComponent Object Reference") (OtherActor :type "Actor Object Reference") (OtherComp :type "PrimitiveComponent Object Reference") (OtherBodyIndex :type Integer))
  (if (== (`self.InitialState`) 1)
    (`PrimitiveComponent.SetCollisionEnabled` (`self.StaticMesh`) "NoCollision")))

(fn `UserConstructionScript`)