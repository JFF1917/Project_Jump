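; BP_Overturn is an actor that periodically flips its BasePlat component over, apparently as an overturning platform.
; After an initial delay on BeginPlay, a looping timer fires the Overturn event at a set period.
; Each call plays one of two timelines, chosen by the AtoB flag, to interpolate relative roll between 0 and 180 degrees.
; Timeline updates set the flag for the opposite direction, so flips alternate.
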(event `self.ReceiveBeginPlay`
  (`KismetSystemLibrary.Delay` (`self.DelayTime`))
  (`KismetSystemLibrary.K2_SetTimerDelegate` (delegate `Overturn`) (`self.PeriodTime`) true))

(event `Overturn`
  (bind _baseplat (`self.BasePlat`))
  (if (`self.AtoB?`)
    (bind (_direction _overturn) (`Timeline|SizeSmall` :!via `PlayFromStart`)
      (:`Update`
        (`SceneComponent.K2_SetRelativeRotation` _baseplat (`KismetMathLibrary.MakeRotator` (`KismetMathLibrary.Lerp` 0.0 180.0 _overturn)) false false)
        (set `self.AtoB?` false)))
    (else
      (bind (_direction_2 _overturn_2) (`Timeline|时间轴` :!via `PlayFromStart`)
        (:`Update`
          (`SceneComponent.K2_SetRelativeRotation` _baseplat (`KismetMathLibrary.MakeRotator` (`KismetMathLibrary.Lerp` 180.0 0.0 _overturn_2)) false false)
          (set `self.AtoB?` true))))))

(fn `UserConstructionScript`)