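; BP_Rotation is an actor that spins three arm components about the vertical axis once play begins.
; BeginPlay calls PlatMove, which starts three separate timelines through a sequence.
; Each timeline's rotation track drives a full-turn yaw Lerp into SetWorldRotation, with SpringArm1 turning opposite to ArmA and SpringArm2.
; World-space rotation keeps each arm's yaw independent of any parent rotation.
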(event `self.ReceiveBeginPlay`
  (`self.PlatMove`))

(event `PlatMove`
  (`|ExecutionSequence`
    (:`then_0`
      (bind (_direction _track_rotation) (`Timeline|时间轴_0`)
        (:`Update`
          (`SceneComponent.K2_SetWorldRotation` (`self.ArmA`) (`KismetMathLibrary.MakeRotator` 0.0 0.0 (`KismetMathLibrary.Lerp` 0.0 360.0 _track_rotation)) false false))))
    (:`then_1`
      (bind (_direction_2 _track_rotation_2) (`Timeline|时间轴_1`)
        (:`Update`
          (`SceneComponent.K2_SetWorldRotation` (`self.SpringArm1`) (`KismetMathLibrary.MakeRotator` 0.0 0.0 (`KismetMathLibrary.Lerp` 0.0 -360.0 _track_rotation_2)) false false))))
    (:`then_2`
      (bind (_direction_3 _track_rotation_3) (`Timeline|时间轴`)
        (:`Update`
          (`SceneComponent.K2_SetWorldRotation` (`self.SpringArm2`) (`KismetMathLibrary.MakeRotator` 0.0 0.0 (`KismetMathLibrary.Lerp` 0.0 360.0 _track_rotation_3)) false false))))))

(fn `UserConstructionScript`)