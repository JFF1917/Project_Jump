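; BP_Tide_Base is an actor that performs a tide-like vertical move once play begins.
; BeginPlay calls Tide, which waits DelayTime times DelayOrder, so instances with different orders can start in a staggered sequence.
; It then caches its location and plays a timeline whose PositionZ track lerps height from the starting Z toward that Z plus OffsetZ, keeping X and Y fixed.
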(event `self.ReceiveBeginPlay`
  (`self.Tide`))

(event `Tide`
  (bind (_returnvalue_x _returnvalue_y _returnvalue_z) (`KismetMathLibrary.BreakVector` (`self.K2_GetActorLocation`)))
  (`KismetSystemLibrary.Delay` (* (`self.DelayTime`) (`self.DelayOrder`)))
  (set `self.Position X` _returnvalue_x)
  (set `self.Position Y` _returnvalue_y)
  (set `self.Position Z` _returnvalue_z)
  (bind (_direction _track_positionz) (`Timeline|时间轴` :!via `PlayFromStart`)
    (:`Update`
      (`self.K2_SetActorLocation` (`KismetMathLibrary.MakeVector` (`self.Position X`) (`self.Position Y`) (`KismetMathLibrary.Lerp` (`self.Position Z`) (+ (`self.Position Z`) (`self.OffsetZ`)) _track_positionz))))))

(fn `UserConstructionScript`)