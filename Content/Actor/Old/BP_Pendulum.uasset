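; BP_Pendulum is a pendulum actor that swings by rotating its BasePillar component around the roll axis.
; On BeginPlay it calls Transverse, which waits DelayTime multiplied by DelayOrder, so instances can start staggered, then plays the Swing timeline from the start.
; The timeline's Overturn track drives a Lerp between A and B that sets the pillar's relative roll, with pitch and yaw held at zero.
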(event `self.ReceiveBeginPlay`
  (`self.Transverse`))

(event `Transverse`
  (`KismetSystemLibrary.Delay` (* (`self.DelayTime`) (`self.DelayOrder`)))
  (bind (_direction _overturn) (`Timeline|Swing` :!via `PlayFromStart`)
    (:`Update`
      (`SceneComponent.K2_SetRelativeRotation` (`self.BasePillar`) (`KismetMathLibrary.MakeRotator` (`KismetMathLibrary.Lerp` (`self.A`) (`self.B`) _overturn)) false false))))

(fn `UserConstructionScript`)