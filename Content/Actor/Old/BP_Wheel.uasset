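; BP_Wheel is an actor that spins its BasePlat component, starting at BeginPlay.
; IsForward selects one of two timelines, each driving a pitch Lerp through a full 360 degrees, forward or backward, with roll fixed at 90.
; DelayAngel times DelayOrder sets the starting angle, so instances can be phase-offset from one another.
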(event `self.ReceiveBeginPlay`
  (`self.Rotate`))

(event `Rotate`
  (bind _returnvalue (* (`self.DelayAngel`) (`self.DelayOrder`)))
  (bind _returnvalue_2 (* (`self.DelayAngel`) (`self.DelayOrder`)))
  (if (`self.IsForward?`)
    (bind (_direction _track_rotation) (`Timeline|时间轴`)
      (:`Update`
        (`SceneComponent.K2_SetRelativeRotation` (`self.BasePlat`) (`KismetMathLibrary.MakeRotator` 90.0 (`KismetMathLibrary.Lerp` _returnvalue_2 (+ _returnvalue_2 360.0) _track_rotation)) false false)))
    (else
      (bind (_direction_2 _track_rotation_2) (`Timeline|时间轴_0`)
        (:`Update`
          (`SceneComponent.K2_SetRelativeRotation` (`self.BasePlat`) (`KismetMathLibrary.MakeRotator` 90.0 (`KismetMathLibrary.Lerp` _returnvalue (- _returnvalue 360.0) _track_rotation_2)) false false))))))

(fn `UserConstructionScript`)