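; Base actor for a tween sector obstacle or effect with Inside, Middle and Outside parts that repeatedly animate their X scale.
; On BeginPlay it caches each part's X scale in Z-named variables and starts a Loop timeline whose events trigger the middle or a random side.
; Each part plays a scale timeline, then a second after a StayTime delay triggered from Update.
; RandomInteger(2) picks Inside or Outside, so the both-sides branch never runs.
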(event `self.ReceiveBeginPlay`
  (bind _returnvalue_x (`KismetMathLibrary.BreakVector` (`SceneComponent.K2_GetComponentScale` (`self.Outside`))))
  (bind _returnvalue_x_2 (`KismetMathLibrary.BreakVector` (`SceneComponent.K2_GetComponentScale` (`self.Inside`))))
  (bind _returnvalue_x_3 (`KismetMathLibrary.BreakVector` (`SceneComponent.K2_GetComponentScale` (`self.Middle`))))
  (set `self.Outside_Z` _returnvalue_x)
  (set `self.Middle_Z` _returnvalue_x_3)
  (set `self.Inside_Z` _returnvalue_x_2)
  (`Timeline|Loop` :!via `PlayFromStart`
    (:`PlayMiddle`
      (`self.PlayMiddle`))
    (:`PlaySide`
      (`self.PlaySide`))))

(event `PlayMiddle`
  (bind (_direction _sizesmall) (`Timeline|SizeBorn` :!via `PlayFromStart`)
    (:`Update`
      (`SceneComponent.SetWorldScale3D` (`self.Middle`) (`KismetMathLibrary.MakeVector` (* (`self.Middle_Z`) _sizesmall) 3.0 1.0))
      (`KismetSystemLibrary.Delay` (`self.StayTime`))
      (bind (_direction_2 _sizesmall_2) (`Timeline|SizeSmall` :!via `PlayFromStart`)
        (:`Update`
          (`SceneComponent.SetWorldScale3D` (`self.Middle`) (`KismetMathLibrary.MakeVector` (* (`self.Middle_Z`) _sizesmall_2) 3.0 1.0)))))))

(event `PlaySide`
  (set `self.RadomInt` (`KismetMathLibrary.RandomInteger` 2))
  (if (== (`self.RadomInt`) 0)
    (`self.PlayInside`)
    (elif (== (`self.RadomInt`) 1)
      (`self.PlayOutside`)
      (else
        (`self.PlayInside`)
        (`self.PlayOutside`)))))

(event `PlayInside`
  (bind (_direction _sizesmall) (`Timeline|时间轴_0` :!via `PlayFromStart`)
    (:`Update`
      (`SceneComponent.SetWorldScale3D` (`self.Inside`) (`KismetMathLibrary.MakeVector` (* (`self.Inside_Z`) _sizesmall) 3.0 1.0))
      (`KismetSystemLibrary.Delay` (`self.StayTime`))
      (bind (_direction_2 _sizesmall_2) (`Timeline|时间轴` :!via `PlayFromStart`)
        (:`Update`
          (`SceneComponent.SetWorldScale3D` (`self.Inside`) (`KismetMathLibrary.MakeVector` (* (`self.Inside_Z`) _sizesmall_2) 3.0 1.0)))))))

(event `PlayOutside`
  (bind (_direction _sizesmall) (`Timeline|时间轴_2` :!via `PlayFromStart`)
    (:`Update`
      (`SceneComponent.SetWorldScale3D` (`self.Outside`) (`KismetMathLibrary.MakeVector` (* (`self.Outside_Z`) _sizesmall) 3.0 1.0))
      (`KismetSystemLibrary.Delay` (`self.StayTime`))
      (bind (_direction_2 _sizesmall_2) (`Timeline|时间轴_1` :!via `PlayFromStart`)
        (:`Update`
          (`SceneComponent.SetWorldScale3D` (`self.Outside`) (`KismetMathLibrary.MakeVector` (* (`self.Outside_Z`) _sizesmall_2) 3.0 1.0)))))))

(fn `UserConstructionScript`)