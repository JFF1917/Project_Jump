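; Base Blueprint for a floating platform actor that animates its BasePlat component up and down along the relative Z axis.
; BeginPlay triggers Float, which waits DelayTime multiplied by DelayOrder, so instances can start in staggered sequence.
; The PlayFloat timeline then plays from the start, using its Overturn track to lerp the Z location between zero and B.
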(event `self.ReceiveBeginPlay`
  (`self.Float`))

(event `Float`
  (`KismetSystemLibrary.Delay` (* (`self.DelayTime`) (`self.DelayOrder`)))
  (bind (_direction _overturn) (`Timeline|PlayFloat` :!via `PlayFromStart`)
    (:`Update`
      (`SceneComponent.K2_SetRelativeLocation` (`self.BasePlat`) (`KismetMathLibrary.MakeVector` 0.0 0.0 (`KismetMathLibrary.Lerp` 0.0 (`self.B`) _overturn)) false false))))

(fn `UserConstructionScript`)