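; BP_Sector is an actor with a BasePlat component meant to spin a full turn, offset by DelayAngel times DelayOrder.
; Two timelines lerp its pitch in opposite directions while holding roll at 90 degrees.
; BeginPlay calls Rotate, which branches on IsForward, but neither branch is connected, so the timelines never run and the platform stays still.
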(event `self.ReceiveBeginPlay`
  (`self.Rotate`))

(event `Rotate`
  (if (`self.IsForward?`)
    _))

(fn `UserConstructionScript`)