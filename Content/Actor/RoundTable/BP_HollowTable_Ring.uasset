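; BP_HollowTable_Ring is a rotating ring platform that can launch the player.
; On BeginPlay, a timeline drives the yaw of BasePlat.
; LaunchPlayer compares player facing with the obstacle's forward vector, using that vector if they differ enough, otherwise the backward one.
; It blends the weighted choice with player facing, scales it, launches the character with a fixed upward velocity, then calls DeleteIMCPlayerMove on the player.
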(event `self.ReceiveBeginPlay`
  (`self.Rotate`))

(event `Rotate`
  (bind (_direction _track_rotation) (`Timeline|时间轴`)
    (:`Update`
      (`SceneComponent.K2_SetRelativeRotation` (`self.BasePlat`) (`KismetMathLibrary.MakeRotator` 0.0 0.0 (`KismetMathLibrary.Lerp` 0.0 (`self.B`) _track_rotation)) false false))))

(fn `LaunchPlayer`
  (params (ObstacleForward :type "Vector Structure") (ObstacleBackward :type "Vector Structure"))
  (bind _bp_player (`self.BP_Player`))
  (bind (_returnvalue_x _returnvalue_y) (`KismetMathLibrary.BreakVector` (* (+ (* ObstacleBackward (`self.ObstacleWeight`)) (`self.PlayerForward`)) (`self.VelocityXYRate`))))
  (bind (_returnvalue_x_2 _returnvalue_y_2) (`KismetMathLibrary.BreakVector` (* (+ (* ObstacleForward (`self.ObstacleWeight`)) (`self.PlayerForward`)) (`self.VelocityXYRate`))))
  ;[0 0 0] 判定角色接近朝向
  (if (> (`KismetMathLibrary.VSize` (- ObstacleForward (`self.PlayerForward`))) 1.0)
    (`Character.LaunchCharacter` _bp_player (`KismetMathLibrary.MakeVector` _returnvalue_x_2 _returnvalue_y_2 1600.0) true true)
    (else
      (`Character.LaunchCharacter` _bp_player (`KismetMathLibrary.MakeVector` _returnvalue_x _returnvalue_y 1600.0) true true)))
  (`/Game/Player/BP_Player.Delete IMC_PlayerMove` _bp_player))

(fn `UserConstructionScript`)