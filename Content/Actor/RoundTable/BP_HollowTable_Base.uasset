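; Round table hazard base with three obstacles spaced 120 degrees apart, which knock BP_Player into the air on contact.
; A timeline started at BeginPlay lerps each obstacle's yaw to spin it.
; Each capsule overlap calls LaunchPlayer, which picks the obstacle's forward or backward vector by comparison with player facing, blends it with that facing for an overriding launch, then calls DeleteIMCPlayerMove on the player.
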(event `self.ReceiveBeginPlay`
  (`self.Rotate`))

(event `Rotate`
  (bind (_direction _track_rotation) (`Timeline|时间轴`)
    (:`Update`
      (`SceneComponent.K2_SetRelativeRotation` (`self.Obstacle`) (`KismetMathLibrary.MakeRotator` -90.0 0.0 (`KismetMathLibrary.Lerp` 0.0 (`self.B`) _track_rotation)) false false)
      (`SceneComponent.K2_SetRelativeRotation` (`self.Obstacle1`) (`KismetMathLibrary.MakeRotator` -90.0 0.0 (`KismetMathLibrary.Lerp` 120.0 (+ (`self.B`) 120.0) _track_rotation)) false false)
      (`SceneComponent.K2_SetRelativeRotation` (`self.Obstacle2`) (`KismetMathLibrary.MakeRotator` -90.0 0.0 (`KismetMathLibrary.Lerp` -120.0 (- (`self.B`) 120.0) _track_rotation)) false false))))

(event `self.Capsule.OnComponentBeginOverlap`
  (params (OverlappedComponent :type "PrimitiveComponent Object Reference") (OtherActor :type "Actor Object Reference") (OtherComp :type "PrimitiveComponent Object Reference") (OtherBodyIndex :type Integer) (bFromSweep :type Boolean) (SweepResult :type "HitResult Structure (by ref)"))
  (bind _output_get (set `self.ObstacleForward` (`SceneComponent.GetForwardVector` (`self.Obstacle`))))
  (set `self.ObstacleBackward` (- (0.0 0.0 0.0) _output_get))
  (bind _asbp_player (cast `/Game/Player/BP_Player` OtherActor))
  (set `self.BP_Player` _asbp_player)
  (set `self.PlayerForward` (`self.GetActorForwardVector` _asbp_player))
  (`self.LaunchPlayer` (`self.ObstacleForward`) (`self.ObstacleBackward`)))

(event `self.Capsule1.OnComponentBeginOverlap`
  (params (OverlappedComponent :type "PrimitiveComponent Object Reference") (OtherActor :type "Actor Object Reference") (OtherComp :type "PrimitiveComponent Object Reference") (OtherBodyIndex :type Integer) (bFromSweep :type Boolean) (SweepResult :type "HitResult Structure (by ref)"))
  (bind _output_get (set `self.ObstacleForward_2` (`SceneComponent.GetForwardVector` (`self.Obstacle1`))))
  (set `self.ObstacleBackward_2` (- (0.0 0.0 0.0) _output_get))
  (bind _asbp_player (cast `/Game/Player/BP_Player` OtherActor))
  (set `self.BP_Player` _asbp_player)
  (set `self.PlayerForward` (`self.GetActorForwardVector` _asbp_player))
  (`self.LaunchPlayer` (`self.ObstacleForward_2`) (`self.ObstacleBackward_2`)))

(event `self.Capsule2.OnComponentBeginOverlap`
  (params (OverlappedComponent :type "PrimitiveComponent Object Reference") (OtherActor :type "Actor Object Reference") (OtherComp :type "PrimitiveComponent Object Reference") (OtherBodyIndex :type Integer) (bFromSweep :type Boolean) (SweepResult :type "HitResult Structure (by ref)"))
  (bind _output_get (set `self.ObstacleForward_3` (`SceneComponent.GetForwardVector` (`self.Obstacle2`))))
  (set `self.ObstacleBackward_3` (- (0.0 0.0 0.0) _output_get))
  (bind _asbp_player (cast `/Game/Player/BP_Player` OtherActor))
  (set `self.BP_Player` _asbp_player)
  (set `self.PlayerForward` (`self.GetActorForwardVector` _asbp_player))
  (`self.LaunchPlayer` (`self.ObstacleForward_3`) (`self.ObstacleBackward_3`)))

(fn `LaunchPlayer`
  (params (ObstacleForward :type "Vector Structure") (ObstacleBackward :type "Vector Structure"))
  (bind _bp_player (`self.BP_Player`))
  (bind (_returnvalue_x _returnvalue_y) (`KismetMathLibrary.BreakVector` (* (+ (* ObstacleBackward (`self.ObstacleWeight`)) (`self.PlayerForward`)) (`self.VelocityXYRate`))))
  (bind (_returnvalue_x_2 _returnvalue_y_2) (`KismetMathLibrary.BreakVector` (* (+ (* ObstacleForward (`self.ObstacleWeight`)) (`self.PlayerForward`)) (`self.VelocityXYRate`))))
  ;[0 0 0] 判定角色接近朝向
  (if (> (`KismetMathLibrary.VSize` (- ObstacleForward (`self.PlayerForward`))) 1.0)
    (`Character.LaunchCharacter` _bp_player (`KismetMathLibrary.MakeVector` _returnvalue_x_2 _returnvalue_y_2 1600.0) true true)
    (else
      (`Character.LaunchCharacter` _bp_player (`KismetMathLibrary.MakeVector` _returnvalue_x _returnvalue_y 1600.0) true true)))
  (`/Game/Player/BP_Player.Delete IMC_PlayerMove` _bp_player))

(fn `UserConstructionScript`)