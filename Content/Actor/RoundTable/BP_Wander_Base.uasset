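; BP_Wander_Base is a rotating round-table obstacle that knocks the player into the air on contact.
; A timeline started at BeginPlay drives the relative yaw of CenterAxis.
; On sphere overlap, it compares player and obstacle forward vectors to pick the obstacle's forward or backward direction, blending it with player forward for the launch.
; After the upward launch, it calls DeleteIMCPlayerMove on BP_Player.
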(event `self.ReceiveBeginPlay`
  (`self.Rotate`))

(event `Rotate`
  (bind (_direction _track_rotation) (`Timeline|时间轴`)
    (:`Update`
      (`SceneComponent.K2_SetRelativeRotation` (`self.CenterAxis`) (`KismetMathLibrary.MakeRotator` 0.0 0.0 (`KismetMathLibrary.Lerp` 0.0 (`self.B`) _track_rotation)) false false))))

(event `self.Sphere.OnComponentBeginOverlap`
  (params (OverlappedComponent :type "PrimitiveComponent Object Reference") (OtherActor :type "Actor Object Reference") (OtherComp :type "PrimitiveComponent Object Reference") (OtherBodyIndex :type Integer) (bFromSweep :type Boolean) (SweepResult :type "HitResult Structure (by ref)"))
  (bind _bp_player_0 (`self.BP Player_0`))
  (bind (_returnvalue_x _returnvalue_y) (`KismetMathLibrary.BreakVector` (* (+ (* (`self.ObstacleBackward`) (`self.ObstacleWeight`)) (`self.PlayerForward`)) (`self.VelocityXYRate`))))
  (bind (_returnvalue_x_2 _returnvalue_y_2) (`KismetMathLibrary.BreakVector` (* (+ (* (`self.ObstacleForward`) (`self.ObstacleWeight`)) (`self.PlayerForward`)) (`self.VelocityXYRate`))))
  (`self.Get Obstacle Forward Backward`)
  (bind _asbp_player (cast `/Game/Player/BP_Player` OtherActor))
  (set `self.BP Player_0` _asbp_player)
  (set `self.PlayerForward` (`self.GetActorForwardVector` _asbp_player))
  ;[0 0 0] 判定角色接近朝向
  (if (> (`KismetMathLibrary.VSize` (- (`self.ObstacleForward`) (`self.PlayerForward`))) 1.0)
    (`Character.LaunchCharacter` _bp_player_0 (`KismetMathLibrary.MakeVector` _returnvalue_x_2 _returnvalue_y_2 1600.0) true true)
    (else
      (`Character.LaunchCharacter` _bp_player_0 (`KismetMathLibrary.MakeVector` _returnvalue_x _returnvalue_y 1600.0) true true)))
  (`/Game/Player/BP_Player.Delete IMC_PlayerMove` _bp_player_0))

(fn `Get Obstacle Forward Backward`
  (bind _output_get (set `self.ObstacleForward` (`SceneComponent.GetForwardVector` (`self.Obstacle`))))
  (set `self.ObstacleBackward` (- (0.0 0.0 0.0) _output_get)))

(fn `UserConstructionScript`)