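; BP_Once_Base is a base platform actor that changes size after something hits it.
; A hit on BasePlat waits StayTime, then caches the current world scale.
; The SizeSmall timeline scales the platform by its curve, and on finish starts the SizeBorn timeline, which scales it again from that cached size, apparently a shrink-then-regrow cycle.
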(event `self.ReceiveBeginPlay`)

(event `self.BasePlat.OnComponentHit`
  (params (HitComponent :type "PrimitiveComponent Object Reference") (OtherActor :type "Actor Object Reference") (OtherComp :type "PrimitiveComponent Object Reference") (NormalImpulse :type "Vector Structure") (Hit :type "HitResult Structure (by ref)"))
  (`KismetSystemLibrary.Delay` (`self.StayTime`))
  (set `self.Size` (`SceneComponent.K2_GetComponentScale` (`self.BasePlat`)))
  (bind (_direction _sizesmall) (`Timeline|SizeSmall` :!via `PlayFromStart`)
    (:`Update`
      (`SceneComponent.SetWorldScale3D` (`self.BasePlat`) (* (`self.Size`) _sizesmall)))
    (:`Finished`
      (bind (_direction_2 _sizesmall_2) (`Timeline|SizeBorn` :!via `PlayFromStart`)
        (:`Update`
          (`SceneComponent.SetWorldScale3D` (`self.BasePlat`) (* (`self.Size`) _sizesmall_2)))))))

(fn `UserConstructionScript`)